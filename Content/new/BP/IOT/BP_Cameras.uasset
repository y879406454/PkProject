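; BP_Cameras is an IoT camera marker actor that opens a web dialog when clicked.
; Each tick its icon mesh turns toward the player camera and shows only while the player controller's IsGod is set.
; Clicking the Normal or Abnormal component loads the matching local-network page in a web widget.
; Page events bind to a callback meant to close the dialog or open a MediaPanel widget.
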(event OnClicked(Normal)
  (params (TouchedComponent :type Primitive%20Component%20Object%20Reference) (ButtonPressed :type Key%20Structure :default "None"))
  ;[1 1 1] 点击加载网页内容
  (bind _webinterface (CallFunction|LoadPage "http://10.10.10.71:3030/#/cameradialog"))
  (EventDispatchers|BindEventtoOnInterfaceEvent _webinterface (delegate Custom|pageCall)))

(event OnClicked(Abnormal)
  (params (TouchedComponent :type Primitive%20Component%20Object%20Reference) (ButtonPressed :type Key%20Structure :default "None"))
  ;[1 1 1] 点击加载网页内容
  (bind _webinterface (CallFunction|LoadPage "http://10.10.10.71:3030/#/cameradialogError"))
  (EventDispatchers|BindEventtoOnInterfaceEvent (stale OnClicked(Normal) _webinterface) (delegate Custom|pageCall)))

(event Custom|pageCall
  (params (Name :type Name) (Data :type Json%20Library%20Value%20Structure) (Callback :type Web%20Interface%20Callback%20Structure))
  ;[1 1 1] 点击加载网页内容
  (switch name "None"
    (:closeCameraDialog
      (Widget|RemovefromParent (Variables|Default|GetMyPage)))
    (:openWindow
      (bind _returnvalue (UserInterface|CreateWidget "/Game/test/BP/level_floor/MediaPanel.MediaPanel_C"))
      (UserInterface|Viewport|AddtoViewport _returnvalue 0))))

(event EventTick
  (params (DeltaSeconds :type Float%20%28single-precision%29))
  ;[1 1 1] 图标跟随镜头
  (Transformation|SetWorldRotation (Variables|Debug|GetStaticMeshComponent) (Math|Rotator|FindLookatRotation (Transformation|GetActorLocation self) (Transformation|GetActorLocation (Game|GetPlayerCameraManager 0))) false false)
  (if (Variables|/Game/test/BP/level_floor/MyPlayerControllerc_2.MyPlayerControllerc_2_C|GetIsGod (Variables|Default|GetMyController))
    (Transformation|SetWorldScale3D (Variables|Debug|GetStaticMeshComponent) "2.000000,2.000000,2.000000")
    (else
      (Transformation|SetWorldScale3D (Variables|Debug|GetStaticMeshComponent) "0, 0, 0"))))

(event EventBeginPlay
  ;[1 1 1] 实例化控制器对象
  (bind _returnvalue (Actor|GetActorOfClass "/Game/test/BP/level_floor/MyPlayerControllerc_2.MyPlayerControllerc_2_C"))
  (Variables|Default|SetMyController _returnvalue))

(fn ConstructionScript)

(fn LoadPage
  (params (pageUrl :type String))
  (bind _returnvalue (UserInterface|CreateWidget "/Game/new/BP/Widgets/BP_Camera_Widget.BP_Camera_Widget_C"))
  (bind _output_get (Variables|Default|SetMyPage _returnvalue))
  (Class|WebInterface|LoadURL (Variables|/Game/new/BP/Widgets/BP_Camera_Widget.BP_Camera_Widget_C|GetWebInterface_Camera _output_get) pageUrl)
  (UserInterface|Viewport|AddtoViewport (Variables|Default|GetMyPage) 0)
  (return (Variables|/Game/new/BP/Widgets/BP_Camera_Widget.BP_Camera_Widget_C|GetWebInterface_Camera _output_get)))