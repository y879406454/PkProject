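; BP_DT_A_A is a test actor that moves continuously along Direction at Speed, alternating between straight down and straight up at random intervals.
; Tick offsets the root transform by frame time without sweep, then runs a Delay into a FlipFlop that reverses the vertical direction.
; The delay length is randomized on BeginPlay and rerolled only on each switch to upward, so it is shared between two consecutive waits.
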(event EventTick
  (params (DeltaSeconds :type Float%20%28single-precision%29))
  (bind _defaultsceneroot (Variables|Default|GetDefaultSceneRoot))
  (bind _returnvalue (Transformation|GetWorldTransform _defaultsceneroot))
  (bind (_location _rotation _scale) (Math|Transform|BreakTransform _returnvalue))
  (Transformation|SetActorTransform (Math|Transform|MakeTransform (+ (* (Math|Vector|Normalize (Variables|Default|Getdirection) 0.0) (* (Utilities|Time|GetWorldDeltaSeconds) (Variables|Default|Getspeed))) _location) _rotation _scale))
  (Utilities|FlowControl|Delay (Variables|Default|Getduration_set))
  (Utilities|FlowControl|FlipFlop
    (:A
      (Variables|Default|Setdirection "0, 0,-1.000000"))
    (:B
      (Variables|Default|Setdirection "0, 0,1.000000")
      (Variables|Default|Setduration_set (Math|Random|RandomFloatinRange 1.0 27.0)))))

(event EventBeginPlay
  (Variables|Default|Setduration_set (Math|Random|RandomFloatinRange 1.0 27.0)))

(fn ConstructionScript)