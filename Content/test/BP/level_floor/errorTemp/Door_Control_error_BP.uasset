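; Clickable door access-control error marker that has the player controller display faulty access-control information.
; Clicking either the static mesh or the widget calls the error display function on MyPlayerControllerc_2, found at BeginPlay.
; Each Tick turns the widget toward the player camera and scales it up when the controller's IsGod flag is set, or to zero otherwise.
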(event OnClicked(Widget)
  (params (TouchedComponent :type Primitive%20Component%20Object%20Reference) (ButtonPressed :type Key%20Structure :default "None"))
  (Default|展示错误门禁信息 (Variables|Default|GetmyController)))

(event OnClicked(StaticMeshComponent)
  (params (TouchedComponent :type Primitive%20Component%20Object%20Reference) (ButtonPressed :type Key%20Structure :default "None"))
  (Default|展示错误门禁信息 (Variables|Default|GetmyController)))

(event EventTick
  (params (DeltaSeconds :type Float%20%28single-precision%29))
  (Transformation|SetWorldRotation (Variables|组件|GetWidget) (Math|Rotator|FindLookatRotation (Transformation|GetActorLocation self) (Transformation|GetActorLocation (Game|GetPlayerCameraManager 0))) false false)
  (if (Variables|/Game/test/BP/level_floor/MyPlayerControllerc_2.MyPlayerControllerc_2_C|GetIsGod (Variables|Default|Getcontroller))
    (Transformation|SetWorldScale3D (Variables|组件|GetWidget) "2.000000,2.000000,2.000000")
    (else
      (Transformation|SetWorldScale3D (Variables|组件|GetWidget) "0, 0, 0"))))

(event EventBeginPlay
  (bind _returnvalue (Actor|GetActorOfClass "/Game/test/BP/level_floor/MyPlayerControllerc_2.MyPlayerControllerc_2_C"))
  (Variables|Default|SetmyController _returnvalue)
  (bind _returnvalue_2 (Actor|GetActorOfClass "/Game/test/BP/level_floor/MyPlayerControllerc_2.MyPlayerControllerc_2_C"))
  (Variables|Default|Setcontroller _returnvalue_2))

(fn ConstructionScript)