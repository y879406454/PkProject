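; Clickable IoT air conditioner actor with on (开启), off (关闭) and fault (异常) states.
; InitItem shows the matching visual group by scaling and selects its label widget.
; Tick turns that label toward the camera and spins SMFSYZ while on.
; Clicking any state's mesh or label has the player controller focus the camera on it, but only the on state opens an info panel, initialized by Id.
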(event OnClicked(Widget)
  (params (TouchedComponent :type Primitive%20Component%20Object%20Reference) (ButtonPressed :type Key%20Structure :default "None"))
  (Default|空调视角聚焦 (Variables|Default|GetmyController) self)
  (switch string (Variables|Default|GetcurState)
    (:开启
      (bind _returnvalue (UserInterface|CreateWidget "/Game/test/BP/IOT/Air_Conditioner/BP_UI_TanChang_Air-Conditioning_Normal.BP_UI_TanChang_Air-Conditioning_Normal_C"))
      (bind _output_get (Variables|/Game/test/BP/level_floor/MyPlayerControllerc_2.MyPlayerControllerc_2_C|SetcurFocusAirPanel (Variables|Default|GetmyController) _returnvalue))
      (Default|InitItemData _output_get (Variables|Default|Getid))
      (UserInterface|Viewport|AddtoViewport _output_get 0))))

(event OnClicked(Widget1)
  (params (TouchedComponent :type Primitive%20Component%20Object%20Reference) (ButtonPressed :type Key%20Structure :default "None"))
  (Default|空调视角聚焦 (Variables|Default|GetmyController) self)
  (switch string (Variables|Default|GetcurState)
    (:开启
      (bind _returnvalue (UserInterface|CreateWidget "/Game/test/BP/IOT/Air_Conditioner/BP_UI_TanChang_Air-Conditioning_Normal.BP_UI_TanChang_Air-Conditioning_Normal_C"))
      (bind _output_get (Variables|/Game/test/BP/level_floor/MyPlayerControllerc_2.MyPlayerControllerc_2_C|SetcurFocusAirPanel (Variables|Default|GetmyController) _returnvalue))
      (Default|InitItemData _output_get (Variables|Default|Getid))
      (UserInterface|Viewport|AddtoViewport _output_get 0))))

(event OnClicked(Widget2)
  (params (TouchedComponent :type Primitive%20Component%20Object%20Reference) (ButtonPressed :type Key%20Structure :default "None"))
  (Default|空调视角聚焦 (Variables|Default|GetmyController) self)
  (switch string (Variables|Default|GetcurState)
    (:开启
      (bind _returnvalue (UserInterface|CreateWidget "/Game/test/BP/IOT/Air_Conditioner/BP_UI_TanChang_Air-Conditioning_Normal.BP_UI_TanChang_Air-Conditioning_Normal_C"))
      (bind _output_get (Variables|/Game/test/BP/level_floor/MyPlayerControllerc_2.MyPlayerControllerc_2_C|SetcurFocusAirPanel (Variables|Default|GetmyController) _returnvalue))
      (Default|InitItemData _output_get (Variables|Default|Getid))
      (UserInterface|Viewport|AddtoViewport _output_get 0))))

(event OnClicked(SM_FSK)
  (params (TouchedComponent :type Primitive%20Component%20Object%20Reference) (ButtonPressed :type Key%20Structure :default "None"))
  ;[1 1 1] 查看正常状态信息
  (Default|空调视角聚焦 (Variables|Default|GetmyController) self)
  (switch string (Variables|Default|GetcurState)
    (:开启
      (bind _returnvalue (UserInterface|CreateWidget "/Game/test/BP/IOT/Air_Conditioner/BP_UI_TanChang_Air-Conditioning_Normal.BP_UI_TanChang_Air-Conditioning_Normal_C"))
      (bind _output_get (Variables|/Game/test/BP/level_floor/MyPlayerControllerc_2.MyPlayerControllerc_2_C|SetcurFocusAirPanel (Variables|Default|GetmyController) _returnvalue))
      (Default|InitItemData _output_get (Variables|Default|Getid))
      (UserInterface|Viewport|AddtoViewport _output_get 0))))

(event OnClicked(SM_FSK1)
  (params (TouchedComponent :type Primitive%20Component%20Object%20Reference) (ButtonPressed :type Key%20Structure :default "None"))
  ;[1 1 1] 查看关闭状态信息
  (Default|空调视角聚焦 (Variables|Default|GetmyController) self)
  (switch string (Variables|Default|GetcurState)
    (:开启
      (bind _returnvalue (UserInterface|CreateWidget "/Game/test/BP/IOT/Air_Conditioner/BP_UI_TanChang_Air-Conditioning_Normal.BP_UI_TanChang_Air-Conditioning_Normal_C"))
      (bind _output_get (Variables|/Game/test/BP/level_floor/MyPlayerControllerc_2.MyPlayerControllerc_2_C|SetcurFocusAirPanel (Variables|Default|GetmyController) _returnvalue))
      (Default|InitItemData _output_get (Variables|Default|Getid))
      (UserInterface|Viewport|AddtoViewport _output_get 0))))

(event OnClicked(SM_FSK2)
  (params (TouchedComponent :type Primitive%20Component%20Object%20Reference) (ButtonPressed :type Key%20Structure :default "None"))
  ;[1 1 1] 查看错误状态信息
  (Default|空调视角聚焦 (Variables|Default|GetmyController) self)
  (switch string (Variables|Default|GetcurState)
    (:开启
      (bind _returnvalue (UserInterface|CreateWidget "/Game/test/BP/IOT/Air_Conditioner/BP_UI_TanChang_Air-Conditioning_Normal.BP_UI_TanChang_Air-Conditioning_Normal_C"))
      (bind _output_get (Variables|/Game/test/BP/level_floor/MyPlayerControllerc_2.MyPlayerControllerc_2_C|SetcurFocusAirPanel (Variables|Default|GetmyController) _returnvalue))
      (Default|InitItemData _output_get (Variables|Default|Getid))
      (UserInterface|Viewport|AddtoViewport _output_get 0))))

(event EventBeginPlay
  (Variables|Default|SetcurWidget (Variables|Default|GetWidget))
  (bind _returnvalue (Actor|GetActorOfClass "/Game/test/BP/level_floor/MyPlayerControllerc_2.MyPlayerControllerc_2_C"))
  (bind _output_get (Variables|Default|SetmyController _returnvalue))
  (Input|EnableInput _output_get))

(event EventTick
  (params (DeltaSeconds :type Float%20%28single-precision%29))
  ;[1 1 1] 标签跟随镜头
  (Transformation|SetWorldRotation (Variables|Default|GetcurWidget) (Math|Rotator|FindLookatRotation (Transformation|GetActorLocation self) (Transformation|GetActorLocation (Game|GetPlayerCameraManager 0))) false false)
  (if (Utilities|Enum|Equal(Enum) (Variables|Default|GetcurState) "开启")
    (Transformation|AddLocalRotation (Variables|Default|GetSM_FSYZ) "0,10.000000, 0" false false)))

(fn ConstructionScript)

(fn InitItem
  (params (state :type String))
  (bind _output_get (Variables|Default|SetcurState state))
  (switch string _output_get
    (:关闭
      (Transformation|SetWorldScale3D (Variables|Default|GetNormal) "0, 0, 0")
      (Transformation|SetWorldScale3D (Variables|Default|GetWarning) "0, 0, 0")
      (Transformation|SetWorldScale3D (Variables|Default|GetClose) "1.000000,1.000000,1.000000")
      (Variables|Default|SetcurWidget (Variables|Default|GetWidget1)))
    (:开启
      (Transformation|SetWorldScale3D (Variables|Default|GetNormal) "1.000000,1.000000,1.000000")
      (Transformation|SetWorldScale3D (Variables|Default|GetWarning) "0, 0, 0")
      (Transformation|SetWorldScale3D (Variables|Default|GetClose) "0, 0, 0")
      (Variables|Default|SetcurWidget (Variables|Default|GetWidget)))
    (:异常
      (Transformation|SetWorldScale3D (Variables|Default|GetNormal) "0, 0, 0")
      (Transformation|SetWorldScale3D (Variables|Default|GetWarning) "1.000000,1.000000,1.000000")
      (Transformation|SetWorldScale3D (Variables|Default|GetClose) "0, 0, 0")
      (Variables|Default|SetcurWidget (Variables|Default|GetWidget2)))))